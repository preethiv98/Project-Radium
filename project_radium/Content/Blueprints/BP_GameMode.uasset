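; BP_GameMode is a game mode that sets up the HUD and spawns AI characters when play begins.
; It adds the Game_UI widget to the viewport, then runs the EQS_FindMoveTo query with itself as querier, picking randomly from the best 25% of results.
; On query success, it spawns a BP_AdvancedAI at each returned location, adjusting for collisions, and draws a temporary debug sphere there.
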(event `self.ReceiveBeginPlay`
  (bind _returnvalue (`|CreateWidget` "/Game/UI/Game_UI.Game_UI_C"))
  (`UserWidget.AddToViewport` _returnvalue 0)
  (bind _returnvalue_2 (`EnvQueryManager.RunEQSQuery` "/Game/Enemies/EQS_FindMoveTo.EQS_FindMoveTo" self "RandomBest25Pct"))
  (add `EnvQueryInstanceBlueprintWrapper.OnQueryFinishedEvent` _returnvalue_2 (delegate `OnQueryFinishedEvent_Event_0`)))

(event `OnQueryFinishedEvent_Event_0`
  (params (QueryInstance :type "EnvQueryInstanceBlueprintWrapper Object Reference") (QueryStatus :type "EEnvQueryStatus Enum" :default "Processing"))
  (switch `EEnvQueryStatus` QueryStatus
    (:`Success`
      (bind _resultlocations (`EnvQueryInstanceBlueprintWrapper.GetQueryResultsAsLocations` QueryInstance))
      (for _array_element _resultlocations
        (`KismetSystemLibrary.DrawDebugSphere` _array_element 100.0 12 (struct :`R` 0.984243 :`G` 1.0 :`A` 1.0) 2.0 2.0)
        (`|SpawnActorFromClass` "/Game/Enemies/BP_AdvancedAI.BP_AdvancedAI_C" (`KismetMathLibrary.MakeTransform` _array_element) "AdjustIfPossibleButDontSpawnIfColliding" "OverrideRootScale" null null)))))

(fn `UserConstructionScript`)