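; Player character Blueprint that spawns a lantern on its mesh socket and handles jump animations, charged attacks and AI interaction.
; Holding left mouse or right trigger replays a windup montage on Tick; only mouse release plays the attack.
; Overlapping an eligible BP_AdvancedAI lets E set its blackboard to permanently stop and clear gotHit.
; CastAttack and hold-time measurement are disconnected, and trigger release only prints debug text.
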(event `self.ReceiveBeginPlay`
  (bind _returnvalue (`|SpawnActorFromClass` "/Game/Blueprints/BP_Lantern.BP_Lantern_C" (`KismetMathLibrary.MakeTransform` (0.0 0.0 0.0)) "AlwaysSpawn" "OverrideRootScale" self null))
  (set `self.CurrentWeapon` _returnvalue)
  (`self.K2_AttachToComponent` _returnvalue (`self.Mesh`) "Lantern" "SnapToTarget" "SnapToTarget" "SnapToTarget" true))

(event `self.ReceiveActorBeginOverlap`
  (params (OtherActor :type "Actor Object Reference"))
  (bind _asbp_advanced_ai (cast `/Game/Enemies/BP_AdvancedAI` OtherActor))
  (if (`/Game/Enemies/BP_AdvancedAI.canpressE` _asbp_advanced_ai)
    (`KismetSystemLibrary.PrintString` "yay I can set E!")
    (set `self.completedBranch` true)))

(event `Key|LeftMouseButton`
  (params (Key :type "Key Structure")))

(event `self.ReceiveTick`
  (params (DeltaSeconds :type "Float (single-precision)"))
  (if (`self.isCharging`)
    (`|PlayMontage` (`self.Mesh`) "/Game/Animations/WindupCW_Montage.WindupCW_Montage")))

(event `Key|SpaceBar`
  (params (Key :type "Key Structure"))
  (:`Pressed`
    (if (`NavMovementComponent.IsFalling` (`self.CharacterMovement`))
      (`|PlayMontage` (`self.Mesh`) "/Game/Animations/Jump_Montage.Jump_Montage")
      (else
        (`|PlayMontage` (`self.Mesh`) "/Game/Animations/Jump_Start_Montage.Jump_Start_Montage"))))
  (:`Released`
    (`|PlayMontage` (`self.Mesh`) "/Game/Animations/JumpEnd_Montage.JumpEnd_Montage")))

(event `self.ReceiveActorEndOverlap`
  (params (OtherActor :type "Actor Object Reference"))
  (set `self.completedBranch` false))

(event `Key|E`
  (params (Key :type "Key Structure"))
  (:`Pressed`
    (if (`self.completedBranch`)
      (`BlackboardComponent.SetValueAsBool` (`AIBlueprintHelperLibrary.GetBlackboard` (stale `self.ReceiveActorBeginOverlap` _asbp_advanced_ai)) "gotHit" false)
      (`BlackboardComponent.SetValueAsBool` (`AIBlueprintHelperLibrary.GetBlackboard` (stale `self.ReceiveActorBeginOverlap` _asbp_advanced_ai)) "permanentStop" true))))

(event `Key|LeftMouseButton`
  (params (Key :type "Key Structure"))
  (:`Pressed`
    (set `self.isCharging` true))
  (:`Released`
    (set `self.isCharging` false)
    (`|PlayMontage` (`self.Mesh`) "/Game/Animations/AttackCW_Montage.AttackCW_Montage")))

(event `Key|Gamepad_RightTrigger`
  (params (Key :type "Key Structure")))

(event `Key|LeftMouseButton`
  (params (Key :type "Key Structure")))

(event `Key|Gamepad_RightTrigger`
  (params (Key :type "Key Structure"))
  (:`Pressed`
    (set `self.isCharging` true))
  (:`Released`
    (set `self.isCharging` false)
    (`KismetSystemLibrary.PrintString` (`KismetStringLibrary.Concat_StrStr` "You held 'Right Trigger for'" (`KismetStringLibrary.Conv_DoubleToString` (`self.holdTime_0`)) " seconds"))))

(fn `UserConstructionScript`)