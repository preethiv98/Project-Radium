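; Enemy AI that follows the player through a behavior tree and becomes eligible for an on-screen purify prompt once hit.
; An actor overlap starts BT_FollowPlayer, while AI perception writes player visibility to the blackboard.
; Point damage sets Purified and the gotHit key, with debug output.
; EnemyRadius overlaps then show the PressEToPurify widget and set CanpressE, though this Blueprint handles no key input.
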(event `self.ReceiveBeginPlay`
  (cast `/Game/Blueprints/BP_CharacterPawn` (`GameplayStatics.GetPlayerPawn` 0))
  (bind _returnvalue (`|CreateWidget` "/Game/UI/PressEToPurify.PressEToPurify_C"))
  (set `self.PurifyWidget` _returnvalue))

(event `self.ReceiveActorBeginOverlap`
  (params (OtherActor :type "Actor Object Reference"))
  (`AIController.RunBehaviorTree` (`AIBlueprintHelperLibrary.GetAIController` self) "/Game/Enemies/BT_FollowPlayer.BT_FollowPlayer")
  (`BlackboardComponent.SetValueAsVector` (`AIBlueprintHelperLibrary.GetBlackboard` self) "TargetDestination" (0.0 0.0 0.0)))

(event `self.AIPerception.OnTargetPerceptionUpdated`
  (params (Actor :type "Actor Object Reference") (Stimulus :type "AIStimulus Structure"))
  (cast `/Game/Blueprints/BP_CharacterPawn` Actor)
  (`BlackboardComponent.SetValueAsBool` (`AIBlueprintHelperLibrary.GetBlackboard` null) "CanSeePlayer" (`.bSuccessfullySensed` (break `AIStimulus` Stimulus)))
  (`KismetSystemLibrary.PrintString` "I see you!"))

(event `self.EnemyRadius.OnComponentBeginOverlap`
  (params (OverlappedComponent :type "PrimitiveComponent Object Reference") (OtherActor :type "Actor Object Reference") (OtherComp :type "PrimitiveComponent Object Reference") (OtherBodyIndex :type Integer) (bFromSweep :type Boolean) (SweepResult :type "HitResult Structure (by ref)"))
  (if (`self.purified`)
    (`UserWidget.AddToViewport` (`self.PurifyWidget`) 0)
    (set `self.canpressE` true)
    (`KismetSystemLibrary.PrintString` "Yay I can pres E!")
    (else
      (cast `/Game/Blueprints/BP_CharacterPawn` OtherActor)
      (`Widget.RemoveFromParent` (`self.PurifyWidget`))
      (`Widget.RemoveFromParent` (stale `self.ReceiveBeginPlay` _returnvalue))
      (set `self.canpressE` false))))

(event `self.ReceiveActorEndOverlap`
  (params (OtherActor :type "Actor Object Reference"))
  (`Widget.RemoveFromParent` (`self.PurifyWidget`))
  (`Widget.RemoveFromParent` (stale `self.ReceiveBeginPlay` _returnvalue))
  (cast `/Game/Blueprints/BP_CharacterPawn` OtherActor)
  (set `self.canpressE` false))

(event `self.ReceivePointDamage`
  (params (Damage :type "Float (single-precision)") (DamageType :type "DamageType Object Reference") (HitLocation :type "Vector Structure") (HitNormal :type "Vector Structure") (HitComponent :type "PrimitiveComponent Object Reference") (BoneName :type Name) (ShotFromDirection :type "Vector Structure") (InstigatedBy :type "Controller Object Reference") (DamageCauser :type "Actor Object Reference") (HitInfo :type "HitResult Structure (by ref)"))
  (`KismetSystemLibrary.DrawDebugSphere` HitLocation 100.0 12 (struct :`R` 1.0 :`G` 0.782468 :`A` 1.0) 1.0 1.0)
  (`KismetSystemLibrary.PrintString` "printed debug sphere!!!" true true (struct :`R` 1.0 :`B` 0.64433 :`A` 1.0))
  (set `self.purified` true)
  (`BlackboardComponent.SetValueAsBool` (`AIBlueprintHelperLibrary.GetBlackboard` null) "gotHit" true))

(fn `UserConstructionScript`)